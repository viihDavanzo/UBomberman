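; Base bomb for a two-player Bomberman-style game, exploding in a cross-shaped blast.
; ExplodeBomb rotates an arrow to fire four capsule traces scaled by the blast multiplier, with debug drawing, collecting players and destructibles and recursively detonating other bombs hit.
; Player hits report a draw or the opponent's score to the game instance.
; Otherwise it destroys the destructibles, returns a bomb to the instigator's count and destroys itself.
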(fn `ExplodeBomb`
  (params (instigator :type "/Game/ThirdPersonCPP/Blueprints/ThirdPersonCharacter Object Reference"))
  (bind _arrow (`self.Arrow`))
  (bind _returnvalue (`SceneComponent.K2_GetComponentLocation` _arrow))
  (bind _asubomberman_game_instance (cast `/Game/WorldSettings/UBomberman_GameInstance` (`GameplayStatics.GetGameInstance`) :!pure true))
  (set `self.bombInstigator` instigator)
  (for _index (range 4)
    (`SceneComponent.K2_AddWorldRotation` (`self.Arrow`) (`KismetMathLibrary.MakeRotator` 0.0 0.0 (* _index 90.0)) false false)
    (bind _outhits (`KismetSystemLibrary.CapsuleTraceMulti` _returnvalue (+ _returnvalue (* (`SceneComponent.GetForwardVector` _arrow) (* (`self.bombBlastMultiplier`) 180.0))) 40.0 0.0 "TraceTypeQuery3" false (`self.actorsToIgnore`) "ForDuration" true (struct :`R` 1.0 :`A` 1.0) (struct :`G` 1.0 :`A` 1.0) 3.0))
    (for _array_element _outhits
      (bind (_bblockinghit _binitialoverlap _time _location _impactpoint _normal _impactnormal _physmat _hitactor) (`GameplayStatics.BreakHitResult` _array_element))
      (cast `/Game/ThirdPersonCPP/Blueprints/Player1_BP` _hitactor
        (:`then`
          (`KismetArrayLibrary.Array_AddUnique` (`self.playersFound`) _hitactor :!label _label))
        (:`CastFailed`
          (cast `/Game/ThirdPersonCPP/Blueprints/Player2_BP` _hitactor
            (:`then`
              (goto _label))
            (:`CastFailed`
              (cast `/Game/Blueprints/Destructable_Master_BP` _hitactor
                (:`then`
                  (`KismetArrayLibrary.Array_AddUnique` (`self.actorsToDestroy`) _hitactor))
                (:`CastFailed`
                  (bind _asbomb_master_bp (cast `/Game/Blueprints/Bomb_Master_BP` _hitactor))
                  (`KismetArrayLibrary.Array_Add` (`/Game/Blueprints/Bomb_Master_BP.actorsToIgnore` _asbomb_master_bp) self)
                  (`self.ExplodeBomb` _asbomb_master_bp (`self.bombInstigator`))))))))))
  (if (> (`KismetArrayLibrary.Array_Length` (`self.playersFound`)) 0)
    (if (== (`KismetArrayLibrary.Array_Length` (`self.playersFound`)) 2)
      (`/Game/WorldSettings/UBomberman_GameInstance.Draw` _asubomberman_game_instance)
      (else
        (cast `/Game/ThirdPersonCPP/Blueprints/Player1_BP` (`|GetArrayItem` (`self.playersFound`))
          (:`then`
            (`/Game/WorldSettings/UBomberman_GameInstance.Player2 Scored` _asubomberman_game_instance))
          (:`CastFailed`
            (`/Game/WorldSettings/UBomberman_GameInstance.Player1 Scored` _asubomberman_game_instance)))))
    (else
      (for _array_element_2 (`self.actorsToDestroy`)
        (`/Engine/EditorBlueprintResources/StandardMacros.IsValid` _array_element_2
          (:`Is Valid`
            (`self.K2_DestroyActor` _array_element_2))))
      (`/Engine/EditorBlueprintResources/StandardMacros.IsValid` (`self.bombInstigator`)
        (:`Is Valid`
          (`/Engine/EditorBlueprintResources/StandardMacros.IncrementInt` (`/Game/ThirdPersonCPP/Blueprints/ThirdPersonCharacter.bombCount` (`self.bombInstigator`))
            (:`  `
              _)))
        (:`Is Not Valid`
          _))
      (`self.K2_DestroyActor` self))))

(fn `UserConstructionScript`)